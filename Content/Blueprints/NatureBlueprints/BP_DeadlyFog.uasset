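; Deadly fog hazard actor that kills the player character if it stays inside the fog too long.
; A swept begin overlap enables Tick, which shows the warning widget and uses a one-second Delay to decrement the character's Seconds counter.
; Below zero, it shows the death widget, destroys the character and frees the cursor.
; Ending overlap hides the warning, resets the counter and disables Tick.
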(event OnComponentBeginOverlap(CollisionComponent)
  (params (OverlappedComponent :type Primitive%20Component%20Object%20Reference) (OtherActor :type Actor%20Object%20Reference) (OtherComp :type Primitive%20Component%20Object%20Reference) (OtherBodyIndex :type Integer) (bFromSweep :type Boolean) (SweepResult :type Hit%20Result%20Structure%20%28by%20ref%29))
  (bind _returnvalue (Game|GetPlayerController 0))
  (Actor|Tick|SetActorTickEnabled bFromSweep)
  (if bFromSweep
    (bind _asthird_person_character (Utilities|Casting|CastToThirdPersonCharacter (Game|GetPlayerCharacter 0)))
    (Variables|/Game/ThirdPersonCPP/Blueprints/ThirdPersonCharacter.ThirdPersonCharacter_C|SetDeadlyFogWidgetVisible _asthird_person_character true)
    (Utilities|FlowControl|Delay 1.0)
    ;[1 1 1] CountDown
    (Variables|/Game/ThirdPersonCPP/Blueprints/ThirdPersonCharacter.ThirdPersonCharacter_C|SetSeconds _asthird_person_character (- (Variables|/Game/ThirdPersonCPP/Blueprints/ThirdPersonCharacter.ThirdPersonCharacter_C|GetSeconds _asthird_person_character) 1))
    (if (< (Variables|/Game/ThirdPersonCPP/Blueprints/ThirdPersonCharacter.ThirdPersonCharacter_C|GetSeconds _asthird_person_character) 0)
      ;[1 1 1] Die
      (bind _asthird_person_character_2 (Utilities|Casting|CastToThirdPersonCharacter (Game|GetPlayerCharacter 0)))
      (Variables|/Game/ThirdPersonCPP/Blueprints/ThirdPersonCharacter.ThirdPersonCharacter_C|SetYouDeadWidgetVisible _asthird_person_character_2 true)
      (Actor|DestroyActor _asthird_person_character_2)
      (Input|SetInputModeGameandUI _returnvalue 0 "DoNotLock" false)
      (Variables|/Script/Engine.PlayerController|SetbShowMouseCursor _returnvalue true))))

(event OnComponentEndOverlap(CollisionComponent)
  (params (OverlappedComponent :type Primitive%20Component%20Object%20Reference) (OtherActor :type Actor%20Object%20Reference) (OtherComp :type Primitive%20Component%20Object%20Reference) (OtherBodyIndex :type Integer))
  (bind _asthird_person_character (Utilities|Casting|CastToThirdPersonCharacter OtherActor))
  (Variables|/Game/ThirdPersonCPP/Blueprints/ThirdPersonCharacter.ThirdPersonCharacter_C|SetDeadlyFogWidgetVisible _asthird_person_character false)
  (Variables|/Game/ThirdPersonCPP/Blueprints/ThirdPersonCharacter.ThirdPersonCharacter_C|SetSeconds _asthird_person_character 5)
  (Actor|Tick|SetActorTickEnabled false))

(event EventBeginPlay
  (bind _returnvalue (UserInterface|CreateWidget "/Game/Blueprints/NatureBlueprints/BP_DeadlyFogWidget.BP_DeadlyFogWidget_C"))
  (UserInterface|Viewport|AddtoViewport _returnvalue 0))

(event EventTick
  (params (DeltaSeconds :type Float%20%28single-precision%29))
  (bind _returnvalue (Game|GetPlayerController 0))
  (if (stale OnComponentBeginOverlap(CollisionComponent) bFromSweep)
    (bind _asthird_person_character (Utilities|Casting|CastToThirdPersonCharacter (Game|GetPlayerCharacter 0)))
    (Variables|/Game/ThirdPersonCPP/Blueprints/ThirdPersonCharacter.ThirdPersonCharacter_C|SetDeadlyFogWidgetVisible _asthird_person_character true)
    (Utilities|FlowControl|Delay 1.0)
    ;[1 1 1] CountDown
    (Variables|/Game/ThirdPersonCPP/Blueprints/ThirdPersonCharacter.ThirdPersonCharacter_C|SetSeconds _asthird_person_character (- (Variables|/Game/ThirdPersonCPP/Blueprints/ThirdPersonCharacter.ThirdPersonCharacter_C|GetSeconds _asthird_person_character) 1))
    (if (< (Variables|/Game/ThirdPersonCPP/Blueprints/ThirdPersonCharacter.ThirdPersonCharacter_C|GetSeconds _asthird_person_character) 0)
      ;[1 1 1] Die
      (bind _asthird_person_character_2 (Utilities|Casting|CastToThirdPersonCharacter (Game|GetPlayerCharacter 0)))
      (Variables|/Game/ThirdPersonCPP/Blueprints/ThirdPersonCharacter.ThirdPersonCharacter_C|SetYouDeadWidgetVisible _asthird_person_character_2 true)
      (Actor|DestroyActor _asthird_person_character_2)
      (Input|SetInputModeGameandUI _returnvalue 0 "DoNotLock" false)
      (Variables|/Script/Engine.PlayerController|SetbShowMouseCursor _returnvalue true))))

(fn ConstructionScript)